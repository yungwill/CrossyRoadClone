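; GrassBlock is a grass floor tile that chains into the endless path of a Crossy Road-style game.
; Its construction script adds two child actors, one at a random rock point and one at a random small-tree point, each chosen from three markers.
; When the player overlaps EndTrigger, it asks CrossyRoadMode to add a floor block, then destroys itself after a short delay.
; GetAttachTransform exposes the AttachPoint world transform.
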(event OnComponentBeginOverlap(EndTrigger)
  (params (OverlappedComponent :type Primitive%20Component%20Object%20Reference) (OtherActor :type Actor%20Object%20Reference) (OtherComp :type Primitive%20Component%20Object%20Reference) (OtherBodyIndex :type Integer) (bFromSweep :type Boolean) (SweepResult :type Hit%20Result%20Structure%20%28by%20ref%29))
  (Utilities|Casting|CastToPlayerChar OtherActor)
  (bind _ascrossy_road_mode (Utilities|Casting|CastToCrossyRoadMode (Game|GetGameMode)))
  (Default|AddFloorBlock _ascrossy_road_mode)
  (Utilities|FlowControl|Delay 6.0)
  (Actor|DestroyActor))

(event EventBeginPlay)

(event Collision|EventActorBeginOverlap
  (params (OtherActor :type Actor%20Object%20Reference)))

(event EventTick
  (params (DeltaSeconds :type Float%20%28single-precision%29)))

(fn ConstructionScript
  (CallFunction|SetSpawnPoints)
  (CallFunction|SetSTreeSpawnPts)
  (CallFunction|SpawnRocks)
  (CallFunction|SpawnSTrees))

(fn GetAttachTransform
  (return (Transformation|GetWorldTransform (Variables|Default|GetAttachPoint))))

(fn SetSpawnPoints
  (Variables|Default|SetRockSpawnPoints (Utilities|Array|MakeArray (Transformation|GetRelativeTransform (Variables|Default|GetSpawnRockL)) (Transformation|GetRelativeTransform (Variables|Default|GetSpawnRock)) (Transformation|GetRelativeTransform (Variables|Default|GetSpawnRockR)))))

(fn SpawnRocks
  (bind _rockspawnpoints (Variables|Default|GetRockSpawnPoints))
  (AddComponent|AddChildActorComponent false (Utilities|Array|Get(acopy) _rockspawnpoints (Math|Random|RandomIntegerinRange 0 (Utilities|Array|LastIndex _rockspawnpoints)))))

(fn SetSTreeSpawnPts
  (Variables|Default|SetSTreeSpawnPts (Utilities|Array|MakeArray (Transformation|GetRelativeTransform (Variables|Default|GetSpawnSmallTreeL)) (Transformation|GetRelativeTransform (Variables|Default|GetSpawnSmallTree)) (Transformation|GetRelativeTransform (Variables|Default|GetSpawnSmallTreeR)))))

(fn SpawnSTrees
  (bind _streespawnpts (Variables|Default|GetSTreeSpawnPts))
  (AddComponent|AddChildActorComponent false (Utilities|Array|Get(acopy) _streespawnpts (Math|Random|RandomIntegerinRange 0 (Utilities|Array|LastIndex _streespawnpts)))))