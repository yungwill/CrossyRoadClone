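; Player character for a Crossy Road-style game, with a random animal mesh picked at construction.
; Axis input moves it in short offsets throttled by DoOnce and a brief delay, while each W press adds score through CrossyRoadMode.
; Death spawns an explosion, triggers the game mode's respawn, destroys GrassBlock actors and itself.
; Its SaveGame step copies the saved high score into the game mode and re-saves the unchanged slot object.
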(event Custom|Death
  ;[1 1 1] Death
  (Input|DisableInput 0)
  (Effects|SpawnEmitteratLocation "/Game/StarterContent/Particles/P_Explosion.P_Explosion" (Transformation|GetActorLocation))
  (Utilities|FlowControl|Delay 0.1)
  (Default|Respawn (Variables|Default|GetGameMode))
  (bind _outactors (Actor|GetAllActorsOfClass "/Game/Blueprints/GrassBlock.GrassBlock_C"))
  (Actor|DestroyActor _outactors)
  (CallFunction|SaveGame)
  (Actor|DestroyActor))

(event EventBeginPlay
  (bind _ascrossy_road_mode (Utilities|Casting|CastToCrossyRoadMode (Game|GetGameMode)))
  (bind _output_get (Variables|Default|SetGameMode _ascrossy_road_mode))
  (Variables|/Game/Blueprints/CrossyRoadMode.CrossyRoadMode_C|SetSpawnTransform _output_get (Transformation|GetActorTransform)))

(event Collision|EventActorBeginOverlap
  (params (OtherActor :type Actor%20Object%20Reference)))

(event Input|AxisEvents|InputAxisFoward
  (params (AxisValue :type Float%20%28single-precision%29))
  (Utilities|FlowControl|DoOnce false :!label _label
    (:Completed
      (Transformation|AddActorWorldOffset (Math|Vector|MakeVector (* AxisValue 27.0) 0.0 0.0))
      (Utilities|FlowControl|Delay 0.1)
      (goto _label Reset))))

(event Input|AxisEvents|InputAxisRight
  (params (AxisValue :type Float%20%28single-precision%29))
  (Utilities|FlowControl|DoOnce false :!label _label
    (:Completed
      (Transformation|AddActorWorldOffset (Math|Vector|MakeVector 0.0 (* AxisValue 27.0) 0.0))
      (Utilities|FlowControl|Delay 0.1)
      (goto _label Reset))))

(event Input|KeyboardEvents|W
  (params (Key :type Key%20Structure))
  (:Pressed
    (bind _ascrossy_road_mode (Utilities|Casting|CastToCrossyRoadMode (Game|GetGameMode)))
    (Default|AddScore _ascrossy_road_mode (Variables|Default|GetPointWorth))))

(fn ConstructionScript
  (CallFunction|RandomizeMesh))

(fn RandomizeMesh
  (bind _character (Variables|Default|GetCharacter))
  (switch int (Math|Random|RandomInteger 4)
    (:Default
      (Components|StaticMesh|SetStaticMesh _character "/Game/Meshes/chicken.chicken" :!label _label))
    (:0
      (goto _label))
    (:1
      (Components|StaticMesh|SetStaticMesh _character "/Game/Meshes/Duck.Duck"))
    (:2
      (Components|StaticMesh|SetStaticMesh _character "/Game/Meshes/Bunny.Bunny"))
    (:3
      (Components|StaticMesh|SetStaticMesh _character "/Game/Meshes/Slug.Slug"))))

(fn SaveGame
  (bind _returnvalue (SaveGame|LoadGamefromSlot "Save1"))
  (bind _output_get (Variables|Default|SetSaveGameObj _returnvalue))
  (bind _assave_game_main (Utilities|Casting|CastToSaveGameMain _output_get))
  (bind _ascrossy_road_mode (Utilities|Casting|CastToCrossyRoadMode (Game|GetGameMode)))
  (Variables|/Game/Blueprints/CrossyRoadMode.CrossyRoadMode_C|SetHighScore _ascrossy_road_mode (Variables|/Game/Blueprints/SaveGameMain.SaveGameMain_C|GetHighScore _assave_game_main))
  (SaveGame|SaveGametoSlot (Variables|Default|GetSaveGameObj) "Save1"))