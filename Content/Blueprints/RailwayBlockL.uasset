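; RailwayBlockL is a railway block Blueprint that keeps spawning trains as child actor components while the game runs.
; Its construction script fills the spawn point list with the relative transform of its SpawnTrain component.
; BeginPlay loops through a random delay of a few seconds, adding a train at a randomly indexed point, currently always that single one.
; Parent BeginPlay is never called, and SpawnSTrees is empty.
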(event EventBeginPlay
  (CallFunction|SpawnTrains :!label _label)
  (Utilities|FlowControl|Delay (Math|Random|RandomFloatinRange 3.0 7.0))
  (goto _label))

(event Collision|EventActorBeginOverlap
  (params (OtherActor :type Actor%20Object%20Reference))
  (|CallParentFunction OtherActor) ; This node is disabled and will not be called.\nDrag off pins to build functionality.
)

(event EventTick
  (params (DeltaSeconds :type Float%20%28single-precision%29))
  (|CallParentFunction DeltaSeconds) ; This node is disabled and will not be called.\nDrag off pins to build functionality.
)

(event EventSpawnSTrees)

(fn ConstructionScript
  (CallFunction|SetTrainSpawnPoints))

(fn SetTrainSpawnPoints
  (Variables|Default|SetTrainSpawnPts (Utilities|Array|MakeArray (Transformation|GetRelativeTransform (Variables|Default|GetSpawnTrain)))))

(fn SpawnTrains
  (bind _trainspawnpts (Variables|Default|GetTrainSpawnPts))
  (AddComponent|AddChildActorComponent false (Utilities|Array|Get(acopy) _trainspawnpts (Math|Random|RandomIntegerinRange 0 (Utilities|Array|LastIndex _trainspawnpts)))))