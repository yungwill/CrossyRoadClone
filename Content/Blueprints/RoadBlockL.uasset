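; RoadBlockL is a road segment Blueprint that keeps spawning traffic, alternating between a vehicle and a truck.
; The construction script fills SpawnPts with a single entry, the relative transform of the SpawnTrain component.
; From BeginPlay, an endless loop adds each one as a child actor component at a transform picked from SpawnPts, with a random delay of a few seconds after every spawn.
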(event EventBeginPlay
  (bind _returnvalue (Math|Random|RandomFloatinRange 2.0 6.0))
  (CallFunction|SpawnVehicle :!label _label)
  (Utilities|FlowControl|Delay _returnvalue)
  (CallFunction|SpawnTruck)
  (Utilities|FlowControl|Delay _returnvalue)
  (goto _label))

(event Collision|EventActorBeginOverlap
  (params (OtherActor :type Actor%20Object%20Reference))
  (|CallParentFunction OtherActor) ; This node is disabled and will not be called.\nDrag off pins to build functionality.
)

(event EventTick
  (params (DeltaSeconds :type Float%20%28single-precision%29))
  (|CallParentFunction DeltaSeconds) ; This node is disabled and will not be called.\nDrag off pins to build functionality.
)

(event EventSpawnSTrees)

(fn ConstructionScript
  (CallFunction|SetVehicleSpawnPoints))

(fn SetVehicleSpawnPoints
  (Variables|Default|SetSpawnPts (Utilities|Array|MakeArray (Transformation|GetRelativeTransform (Variables|Default|GetSpawnTrain)))))

(fn SpawnVehicle
  (bind _spawnpts (Variables|Default|GetSpawnPts))
  (AddComponent|AddChildActorComponent false (Utilities|Array|Get(acopy) _spawnpts (Math|Random|RandomIntegerinRange 0 (Utilities|Array|LastIndex _spawnpts)))))

(fn SpawnTruck
  (bind _spawnpts (Variables|Default|GetSpawnPts))
  (AddComponent|AddChildActorComponent false (Utilities|Array|Get(acopy) _spawnpts (Math|Random|RandomIntegerinRange 0 (Utilities|Array|LastIndex _spawnpts)))))