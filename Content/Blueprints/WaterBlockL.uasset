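; WaterBlockL is a water block Blueprint that repeatedly spawns logs as child actors.
; The construction script stores the SpawnLog component's relative transform as the only entry in the spawn-point array.
; BeginPlay runs an endless loop that adds a log at a randomly picked spawn point, then waits a random few seconds.
; The SpawnSTrees event is empty, and the parent BeginPlay call is never reached.
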(event EventBeginPlay
  (CallFunction|SpawnLogs :!label _label)
  (Utilities|FlowControl|Delay (Math|Random|RandomFloatinRange 3.0 7.0))
  (goto _label))

(event EventTick
  (params (DeltaSeconds :type Float%20%28single-precision%29))
  (|CallParentFunction DeltaSeconds) ; This node is disabled and will not be called.\nDrag off pins to build functionality.
)

(event EventSpawnSTrees)

(fn ConstructionScript
  (CallFunction|SetLogSpawnPoints))

(fn SetLogSpawnPoints
  (Variables|Default|SetLogSpawnPts (Utilities|Array|MakeArray (Transformation|GetRelativeTransform (Variables|Default|GetSpawnLog)))))

(fn SpawnLogs
  (bind _logspawnpts (Variables|Default|GetLogSpawnPts))
  (AddComponent|AddChildActorComponent false (Utilities|Array|Get(acopy) _logspawnpts (Math|Random|RandomIntegerinRange 0 (Utilities|Array|LastIndex _logspawnpts)))))