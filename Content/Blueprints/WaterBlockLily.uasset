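; WaterBlockLily is a water block actor that places a lily at a random position on itself.
; The construction script gathers the relative transforms of four SpawnLily marker components into LilySpawnPts, then adds a child actor component at one chosen at random.
; The event graph holds only disabled default events and an empty SpawnSTrees event.
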(event EventBeginPlay)

(event Collision|EventActorBeginOverlap
  (params (OtherActor :type Actor%20Object%20Reference)))

(event EventTick
  (params (DeltaSeconds :type Float%20%28single-precision%29)))

(event EventSpawnSTrees)

(fn ConstructionScript
  (CallFunction|SetLilySpawnPts)
  (CallFunction|SpawnLily))

(fn SpawnLily
  (bind _lilyspawnpts (Variables|Default|GetLilySpawnPts))
  (AddComponent|AddChildActorComponent false (Utilities|Array|Get(acopy) _lilyspawnpts (Math|Random|RandomIntegerinRange 0 (Utilities|Array|LastIndex _lilyspawnpts)))))

(fn SetLilySpawnPts
  (Variables|Default|SetLilySpawnPts (Utilities|Array|MakeArray (Transformation|GetRelativeTransform (Variables|Default|GetSpawnLily1)) (Transformation|GetRelativeTransform (Variables|Default|GetSpawnLily2)) (Transformation|GetRelativeTransform (Variables|Default|GetSpawnLily3)) (Transformation|GetRelativeTransform (Variables|Default|GetSpawnLily4)))))